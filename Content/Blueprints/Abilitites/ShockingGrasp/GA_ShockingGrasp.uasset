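; GA_ShockingGrasp is a gameplay ability for a melee Shocking Grasp cast by BP_Character.
; After committing, it plays the cast montage on the character's mesh, whose notifies switch MeleeSphere collision between query-only and off to open and close the hit window.
; The ability ends when the montage completes, blends out or is interrupted.
; Hit effects are not handled here, and a MeleeParticles deactivation node is left unconnected.
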(event Ability|EventActivateAbility
  (bind _asbp_character (Utilities|Casting|CastToBP_Character (.OwnerActor (Utilities|Struct|BreakGameplayAbilityActorInfo (Ability|GetActorInfo)))))
  (Variables|Default|SetCharacterRef _asbp_character)
  (bind _returnvalue (Ability|CommitAbility))
  (if _returnvalue
    (bind _notifyname (Animation|Montage|PlayMontage (Variables|/Script/Engine.Character|GetMesh (Variables|Default|GetCharacterRef)) "/Game/RetargetAnims/AIM_CastShockingGrasp.AIM_CastShockingGrasp" 0.8)
      (:OnCompleted
        (Ability|EndAbility :!label _label))
      (:OnBlendOut
        (goto _label))
      (:OnInterrupted
        (goto _label))
      (:OnNotifyBegin
        (if (Utilities|Name|Equal(Name) _notifyname "activateColision")
          (Collision|SetCollisionEnabled (Variables|/Game/Blueprints/Character/BP_Character.BP_Character_C|GetMeleeSphere (Variables|Default|GetCharacterRef)) "QueryOnly")
          (elif (Utilities|Name|Equal(Name) _notifyname "deactivateColision")
            (Collision|SetCollisionEnabled (Variables|/Game/Blueprints/Character/BP_Character.BP_Character_C|GetMeleeSphere (Variables|Default|GetCharacterRef)) "NoCollision")))))))

(event Ability|EventOnEndAbility
  (params (bWasCancelled :type Boolean)))