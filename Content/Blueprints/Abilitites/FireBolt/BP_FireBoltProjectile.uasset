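; Projectile actor for the FireBolt ability, launched by a velocity passed into its projectile movement component.
; Overlapping a BP_Character other than the Instigator applies damage and damage-over-time Gameplay Effects through that character's own Ability System Component, then detonates.
; Blocking hits on the sphere detonate without applying effects.
; Detonation plays an explosion sound and particle at the impact point, then destroys the actor after a short delay.
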(event OnComponentHit(SphereComponent)
  (params (HitComponent :type Primitive%20Component%20Object%20Reference) (OtherActor :type Actor%20Object%20Reference) (OtherComp :type Primitive%20Component%20Object%20Reference) (NormalImpulse :type Vector :default "0, 0, 0") (Hit :type Hit%20Result%20Structure%20%28by%20ref%29))
  (CallFunction|DestroyEvent (.ImpactPoint (Collision|BreakHitResult Hit))))

(event OnComponentBeginOverlap(SphereComponent)
  (params (OverlappedComponent :type Primitive%20Component%20Object%20Reference) (OtherActor :type Actor%20Object%20Reference) (OtherComp :type Primitive%20Component%20Object%20Reference) (OtherBodyIndex :type Integer) (bFromSweep :type Boolean) (SweepResult :type Hit%20Result%20Structure%20%28by%20ref%29))
  (bind _asbp_character (Utilities|Casting|CastToBP_Character OtherActor))
  (if (!= _asbp_character (Variables|Default|GetInstigator))
    (GameplayEffects|ApplyGameplayEffectToSelf :self (Ability|GetAbilitySystemComponent _asbp_character) :GameplayEffectClass "/Game/Blueprints/Abilitites/FireBolt/GE_FireboltDamage.GE_FireboltDamage_C")
    (GameplayEffects|ApplyGameplayEffectToSelf :self (Ability|GetAbilitySystemComponent _asbp_character) :GameplayEffectClass "/Game/Blueprints/Abilitites/FireBolt/GE_Firebolt_DoT.GE_Firebolt_DoT_C")
    (CallFunction|DestroyEvent (.ImpactPoint (Collision|BreakHitResult SweepResult)))))

(event Custom|InitProjectileMovement
  (params (Velocity :type Vector))
  (Variables|/Script/Engine.MovementComponent|SetVelocity (Variables|Default|GetProjectileMovementComponent) Velocity))

(event Custom|DestroyEvent
  (params (DesiredLocation :type Vector))
  (Audio|PlaySoundatLocation "/Game/StarterContent/Audio/Explosion01.Explosion01" DesiredLocation "0, 0, 0" 1.0 1.0 0.0 0 0 0)
  (Effects|SpawnEmitteratLocation "/Game/StarterContent/Particles/P_Explosion.P_Explosion" DesiredLocation)
  (Utilities|FlowControl|Delay 0.2)
  (Actor|DestroyActor))

(fn ConstructionScript)