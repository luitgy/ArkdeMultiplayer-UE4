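; Gameplay ability that casts a firebolt from a BP_Character, cancelling if the cast or commit fails.
; It plays the AIM_CastFirebolt montage while spawning a BP_FireBoltProjectile attached to the character at socket abilityRightSocket.
; A montage notify detaches the projectile and launches it along the character's forward vector at ProjectileSpeed.
; The ability ends when the montage completes, blends out or is interrupted.
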(event Ability|EventActivateAbility
  (bind _asbp_character (Utilities|Casting|CastToBP_Character (.OwnerActor (Utilities|Struct|BreakGameplayAbilityActorInfo (Ability|GetActorInfo))))
    (:then
      (Variables|Default|SetCharacterRef _asbp_character)
      (bind _returnvalue (Ability|CommitAbility))
      (if _returnvalue
        (Animation|Montage|PlayMontage (Variables|/Script/Engine.Character|GetMesh (Variables|Default|GetCharacterRef)) "/Game/RetargetAnims/AIM_CastFirebolt.AIM_CastFirebolt"
          (:then
            (bind _spawnedactor (|SpawnActor :Class "/Game/Blueprints/Abilitites/FireBolt/BP_FireBoltProjectile.BP_FireBoltProjectile_C" :Instigator (Variables|Default|GetCharacterRef))
              (:Success
                (bind _asbp_fire_bolt_projectile (Utilities|Casting|CastToBP_FireBoltProjectile _spawnedactor))
                (bind _output_get (Variables|Default|SetProjectileRef _asbp_fire_bolt_projectile))
                (Transformation|AttachActorToActor _output_get (Variables|Default|GetCharacterRef) "abilityRightSocket" "KeepRelative" "KeepRelative" "KeepRelative" true))))
          (:OnCompleted
            (Ability|EndAbility :!label _label))
          (:OnBlendOut
            (goto _label))
          (:OnInterrupted
            (goto _label))
          (:OnNotifyBegin
            (bind _projectileref (Variables|Default|GetProjectileRef)
              (:then
                (Transformation|DetachFromActor _projectileref "KeepRelative" "KeepRelative" "KeepRelative")
                (Default|InitProjectileMovement (Variables|Default|GetProjectileRef) (* (Transformation|GetActorForwardVector (Variables|Default|GetCharacterRef)) (Variables|Default|GetProjectileSpeed))))
              (:else))))
        (else
          (Ability|CancelAbility))))
    (:CastFailed
      (Ability|CancelAbility))))

(event Ability|EventOnEndAbility
  (params (bWasCancelled :type Boolean)))